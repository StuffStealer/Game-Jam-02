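; Player character that talks to NPCs, keeps an item and token inventory, and has an AI dragon companion.
; Setup spawns the dragon and HUD, and input toggles a dragon interaction view with its own camera target and UI.
; When skill flags allow, a faded toggle switches to flight, hiding the dragon and swapping mesh visibility, camera, movement mode and animation.
; Inventory functions stack items by class and count tokens separately.
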(event `self.Interaction_Zone.OnComponentBeginOverlap`
  (params (OverlappedComponent :type "PrimitiveComponent Object Reference") (OtherActor :type "Actor Object Reference") (OtherComp :type "PrimitiveComponent Object Reference") (OtherBodyIndex :type Integer) (bFromSweep :type Boolean) (SweepResult :type "HitResult Structure (by ref)"))
  (if (`KismetMathLibrary.ClassIsChildOf` (`GameplayStatics.GetObjectClass` OtherActor) "/Game/Blueprints/PNJ/BP_Master_PNJ.BP_Master_PNJ_C")
    (bind _asbp_master_pnj (cast `/Game/Blueprints/PNJ/BP_Master_PNJ` OtherActor))
    (bind _returnvalue (`GameplayStatics.GetActorOfClass` "/Game/Blueprints/PNJ/BP_Master_PNJ.BP_Master_PNJ_C"))
    (`/Game/Blueprints/PNJ/BP_Master_PNJ.Ref_Actor` _returnvalue _asbp_master_pnj)))

(event `self.ReceiveBeginPlay`
  (`self.Setup_Player`))

(event `InputAxisKey|MouseWheelAxis`
  (params (AxisValue :type "Float (single-precision)"))
  (set `SpringArmComponent.TargetArmLength` (`KismetMathLibrary.FClamp` (+ (* AxisValue -150.0) (`SpringArmComponent.TargetArmLength` (`self.SpringArm`))) 800.0 3000.0) (`self.SpringArm`)))

(event `EnhancedInput|/Game/Blueprints/Player/Input/Actions/IA_Interact`
  (params (ActionValue :type Boolean) (ElapsedSeconds :type "Float (double-precision)") (TriggeredSeconds :type "Float (double-precision)") (InputAction :type "InputAction Object Reference" :default "/Game/Blueprints/Player/Input/Actions/IA_Interact.IA_Interact"))
  (:`Started`
    (bind _returnvalue (`GameplayStatics.GetActorOfClass` "/Game/Blueprints/PNJ/BP_Master_PNJ.BP_Master_PNJ_C"))
    (`/Game/Blueprints/PNJ/BP_Master_PNJ.Context_Dialogue` _returnvalue)))

(event `EnhancedInput|/Game/Blueprints/Player/Input/Actions/IA_Interact_With_Dragon`
  (params (ActionValue :type Boolean) (ElapsedSeconds :type "Float (double-precision)") (TriggeredSeconds :type "Float (double-precision)") (InputAction :type "InputAction Object Reference" :default "/Game/Blueprints/Player/Input/Actions/IA_Interact_With_Dragon.IA_Interact_With_Dragon"))
  (:`Started`
    (if (not (`NavMovementComponent.IsFlying` (`self.CharacterMovement`)))
      (`/Engine/EditorBlueprintResources/StandardMacros.FlipFlop` :!label _label
        (:`A`
          (bind _returnvalue (`GameplayStatics.GetActorOfClass` "/Game/Blueprints/Dragon/BP_Master_Dragon.BP_Master_Dragon_C"))
          (`PlayerController.SetViewTargetWithBlend` (`GameplayStatics.GetPlayerController` 0) _returnvalue 0.0 "VTBlend_Linear" 0.0 false)
          (`/Game/Blueprints/Dragon/BP_Master_Dragon.Stop_Movement` _returnvalue)
          (bind _returnvalue_2 (`|CreateWidget` "/Game/Blueprints/Dragon/Widgets/WIB_UI_Interact.WIB_UI_Interact_C"))
          (bind _output_get (set `self.Ref_WIB_Comestic` _returnvalue_2))
          (`UserWidget.AddToViewport` _output_get 0)
          (`WidgetBlueprintLibrary.SetInputMode_GameAndUIEx` (`GameplayStatics.GetPlayerController` 0) _returnvalue_2)
          (set `PlayerController.bShowMouseCursor` true (`GameplayStatics.GetPlayerController` 0)))
        (:`B`
          (`PlayerController.SetViewTargetWithBlend` (`GameplayStatics.GetPlayerController` 0) self 0.0 "VTBlend_Linear" 0.0 false)
          (bind _returnvalue_3 (`GameplayStatics.GetActorOfClass` "/Game/Blueprints/Dragon/BP_Master_Dragon.BP_Master_Dragon_C"))
          (`/Game/Blueprints/Dragon/BP_Master_Dragon.Stop_Movement` _returnvalue_3)
          (`Widget.RemoveFromParent` (`self.Ref_WIB_Comestic`))
          (`WidgetBlueprintLibrary.SetInputMode_GameOnly` (`GameplayStatics.GetPlayerController` 0))
          (set `PlayerController.bShowMouseCursor` false (`GameplayStatics.GetPlayerController` 0))
          (set `self.Ref_WIB_Comestic` null))))))

(event `Remove_UI_Dragon_Interact`
  (goto _label))

(event `EnhancedInput|/Game/Blueprints/Player/Input/Actions/IA_Fly`
  (params (ActionValue :type Boolean) (ElapsedSeconds :type "Float (double-precision)") (TriggeredSeconds :type "Float (double-precision)") (InputAction :type "InputAction Object Reference" :default "/Game/Blueprints/Player/Input/Actions/IA_Fly.IA_Fly"))
  (bind _ref_hud (`self.Ref_HUD`))
  (bind _mesh (`self.Mesh`))
  (bind ((`Can_Fly?_7_3F2BEC46400130C2C9A247AA0BC82E6D` _can_fly_) (`Is_Hungry_14_C97CB7974C9FDED1F65E4F801B6627BF` _is_hungry)) (break `/Game/Blueprints/Player/Struct_Dragon_Skill` (`self.Struct_Skill_Unlock`)))
  (:`Started`
    (if (and _can_fly_ _is_hungry)
      (`self.Ref_WIB_Comestic`
        (:`then`
          (`self.Remove_UI_Dragon_Interact`))
        (:`else`
          _))
      (`UserWidget.PlayAnimation` _ref_hud (`/Game/Blueprints/Player/Widgets/WIB_HUD.FadeInFadeIOut` _ref_hud) 0.0 1 "Forward" 1.0 false)
      (`KismetSystemLibrary.Delay` 1.3)
      (`/Engine/EditorBlueprintResources/StandardMacros.FlipFlop`
        (:`A`
          (`SceneComponent.SetVisibility` (`self.StaticMesh`) true false)
          (`self.SetActorHiddenInGame` (`self.Ref_Dragon`) true)
          (`CharacterMovementComponent.SetMovementMode` (`self.CharacterMovement`) "MOVE_Flying" 0)
          (`ActorComponent.SetActive` (`self.Camera1`) true false)
          (`ActorComponent.SetActive` (`self.Camera`) false false)
          (set `SpringArmComponent.bUsePawnControlRotation` true (`self.SpringArm1`))
          (`SkeletalMeshComponent.SetAnimationMode` _mesh "AnimationSingleNode" true)
          (`SkeletalMeshComponent.PlayAnimation` _mesh "/Game/Assets/Player/Build/Flying.Flying" true)
          (`SkeletalMeshComponent.PlayAnimation` (`self.Mesh`) "/Game/Assets/Player/Build/Flying.Flying" true))
        (:`B`
          (`SceneComponent.SetVisibility` (`self.StaticMesh`) false false)
          (`self.SetActorHiddenInGame` (`self.Ref_Dragon`) false)
          (`CharacterMovementComponent.SetMovementMode` (`self.CharacterMovement`) "MOVE_Walking" 0)
          (`ActorComponent.SetActive` (`self.Camera1`) false false)
          (`ActorComponent.SetActive` (`self.Camera`) true false)
          (set `SpringArmComponent.bUsePawnControlRotation` false (`self.SpringArm1`))
          (`SceneComponent.K2_SetWorldRotation` :`self` (`Actor.RootComponent` (`GameplayStatics.GetPlayerCharacter` 0)))
          (`SceneComponent.K2_SetWorldRotation` :`self` (`Actor.RootComponent` (`GameplayStatics.GetPlayerController` 0)))
          (`SceneComponent.K2_SetWorldRotation` :`self` (`self.SpringArm1`))
          (`SkeletalMeshComponent.SetAnimationMode` (`self.Mesh`) "AnimationBlueprint" true))))))

(event `Key|B`
  (params (Key :type "Key Structure"))
  (:`Pressed`
    (for _array_element (`self.Ref_Struct_Inventory`)
      (bind (_item _item_thumbnail _quantity_item) (break `/Game/Blueprints/Inventory/Struct_Inventory` _array_element))
      (`KismetSystemLibrary.PrintString` (`KismetSystemLibrary.GetDisplayName` _item))
      (`KismetSystemLibrary.PrintString` (`KismetStringLibrary.Conv_IntToString` _quantity_item)))))

(event `EnhancedInput|/Game/Blueprints/Player/Input/Actions/IA_UpDown`
  (params (ActionValue :type "Vector2D Structure") (ElapsedSeconds :type "Float (double-precision)") (TriggeredSeconds :type "Float (double-precision)") (InputAction :type "InputAction Object Reference" :default "/Game/Blueprints/Player/Input/Actions/IA_UpDown.IA_UpDown"))
  (:`Triggered`
    (if (`NavMovementComponent.IsFlying` (`self.CharacterMovement`))
      (`self.AddMovementInput` (`self.GetActorUpVector` (`self.GetController`)) ActionValue_X))))

(fn `Add_Inventory`
  (params (Ref_Item :type "/Game/Blueprints/Inventory/BP_Master_Item Object Reference"))
  (if (`/Game/Blueprints/Inventory/BP_Master_Item.Is_Token?` Ref_Item)
    (`/Engine/EditorBlueprintResources/StandardMacros.IncrementInt` (`self.Token`))
    (else
      (if (`KismetArrayLibrary.Array_IsNotEmpty` (`self.Ref_Struct_Inventory`))
        (for (_array_element _array_index) (`self.Ref_Struct_Inventory`)
          (bind ((`Item_7_AFABEFFA4BFFCF1B996E3EAE3E81E7A7` _item) (`Quantity_Item_5_5421E7DD4F52B09CF7E05D9668D75916` _quantity_item)) (break `/Game/Blueprints/Inventory/Struct_Inventory` _array_element))
          (if (== (`GameplayStatics.GetObjectClass` _item) (`GameplayStatics.GetObjectClass` Ref_Item))
            (bind _result (`/Engine/EditorBlueprintResources/StandardMacros.IncrementInt` _quantity_item)
              (:`  `
                (`KismetArrayLibrary.Array_Set` (`self.Ref_Struct_Inventory`) _array_index (make `/Game/Blueprints/Inventory/Struct_Inventory` Ref_Item (`/Game/Blueprints/Inventory/BP_Master_Item.Thumbnail` Ref_Item) _result))
                (set `self.Item_Not_Add` false)))
            (else
              (set `self.Item_Not_Add` true))))
        (else
          (set `self.Item_Not_Add` true)))
      (if (`self.Item_Not_Add`)
        (`KismetArrayLibrary.Array_Add` (`self.Ref_Struct_Inventory`) (make `/Game/Blueprints/Inventory/Struct_Inventory` Ref_Item (`/Game/Blueprints/Inventory/BP_Master_Item.Thumbnail` Ref_Item) 1))))))

(fn `Remove_Item`
  (params (Ref_Item :type "/Game/Blueprints/Inventory/BP_Master_Item Object Reference"))
  (for _array_element (`self.Ref_Struct_Inventory`)
    (if (== (`GameplayStatics.GetObjectClass` (`.Item_7_AFABEFFA4BFFCF1B996E3EAE3E81E7A7` (break `/Game/Blueprints/Inventory/Struct_Inventory` _array_element))) (`GameplayStatics.GetObjectClass` Ref_Item))
      (`KismetArrayLibrary.Array_RemoveItem` (`self.Ref_Struct_Inventory`) _array_element))))

(fn `Setup_Player`
  (bind _returnvalue (`GameplayStatics.GetPlayerController` 0))
  (bind (_returnvalue_x _returnvalue_y _returnvalue_z) (`KismetMathLibrary.BreakVector` (`SceneComponent.K2_GetComponentLocation` (`self.Mesh`))))
  (`WidgetBlueprintLibrary.SetInputMode_GameOnly` _returnvalue)
  (set `PlayerController.bShowMouseCursor` false _returnvalue)
  (bind _returnvalue_2 (`AIBlueprintHelperLibrary.SpawnAIFromClass` "/Game/Blueprints/Dragon/BP_Master_Dragon.BP_Master_Dragon_C" "/Game/Blueprints/Dragon/BP_BT_Dragon.BP_BT_Dragon" (`KismetMathLibrary.MakeVector` _returnvalue_x _returnvalue_y (+ _returnvalue_z 100.0)) (struct) false null))
  (set `self.Ref_Dragon` _returnvalue_2)
  (bind _returnvalue_3 (`|CreateWidget` "/Game/Blueprints/Player/Widgets/WIB_HUD.WIB_HUD_C"))
  (bind _output_get (set `self.Ref_HUD` _returnvalue_3))
  (`UserWidget.AddToViewport` _output_get 0))

(fn `UserConstructionScript`)