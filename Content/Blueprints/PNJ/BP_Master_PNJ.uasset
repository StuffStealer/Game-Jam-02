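; Master NPC Blueprint that runs quest dialogue and completion when its bound dialogue event fires.
; It matches the interacted actor's class to a DataQuest row for texts and item condition, then steps lines through a WIB_Dialogue widget.
; Holding the exact required item quantity completes the quest, hides its marker, removes the item, and grants a one-time hardcoded skill unlock and pie item.
; Dialogue stops responding once the completion text ends.
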(event `self.ReceiveBeginPlay`
  (add `self.Context_Dialogue` (delegate `Dialogue`)))

(event `Dialogue`
  (if (not (`self.Quest_Finish`))
    (`self.Check_Condition_For_Finish_Quest`)
    (if (`self.Quest_Completed?`)
      (bind (_resultat _text _finish_quest_text) (`self.Check_PNJ`)
        (:`Output`
          (`self.Display_Dialogue` _resultat _finish_quest_text)))
      (else
        (bind (_resultat_2 _text_2) (`self.Check_PNJ`)
          (:`Output`
            (`self.Display_Dialogue` _resultat_2 _text_2)))))))

(event `Check_Condition_For_Finish_Quest`
  (if (not (`self.Is_Check`))
    (bind (_resultat _text _finish_quest_text _condition_for_quest) (`self.Check_PNJ`)
      (:`Output`
        (if _resultat
          (bind _returnvalue (`GameplayStatics.GetActorOfClass` "/Game/Blueprints/Player/BP_Player.BP_Player_C"))
          (for _array_element (`/Game/Blueprints/Player/BP_Player.Ref_Struct_Inventory` _returnvalue)
            (bind ((`Item_7_AFABEFFA4BFFCF1B996E3EAE3E81E7A7` _item) (`Quantity_Item_5_5421E7DD4F52B09CF7E05D9668D75916` _quantity_item)) (break `/Game/Blueprints/Inventory/Struct_Inventory` _array_element))
            (bind (_item_2 _quantity_item_necessary) (break `/Game/Blueprints/PNJ/Struct_Condition_For_Finish_Quest` _condition_for_quest))
            (if (and (== (`GameplayStatics.GetObjectClass` _item) _item_2) (== _quantity_item _quantity_item_necessary))
              (set `self.Quest_Completed?` true)
              (`SceneComponent.SetHiddenInGame` (`/Game/Blueprints/PNJ/BP_Master_PNJ.Quest` (`self.Ref_Actor_Interaction`)) true false)
              (bind _returnvalue_2 (`GameplayStatics.GetActorOfClass` "/Game/Blueprints/Player/BP_Player.BP_Player_C"))
              (`/Game/Blueprints/Player/BP_Player.Remove_Item` _returnvalue_2 _item)
              (`/Engine/EditorBlueprintResources/StandardMacros.DoOnce` false
                (:`Completed`
                  (bind _returnvalue_3 (`GameplayStatics.GetActorOfClass` "/Game/Blueprints/Player/BP_Player.BP_Player_C"))
                  (set `/Game/Blueprints/Player/BP_Player.Struct_Skill_Unlock` (make `/Game/Blueprints/Player/Struct_Dragon_Skill` true) _returnvalue_3)
                  (bind _returnvalue_4 (`|SpawnActorFromClass` "/Game/Blueprints/Inventory/Childs/BP_Item_Pie.BP_Item_Pie_C" (`KismetMathLibrary.MakeTransform` (0.0 0.0 -50.0)) "Undefined" "MultiplyWithRoot" null null))
                  (`/Game/Blueprints/Player/BP_Player.Add_Inventory` _returnvalue_3 _returnvalue_4)
                  (`self.K2_DestroyActor` _returnvalue_4)
                  (set `self.Is_Check` true)))
              (else
                (set `self.Quest_Completed?` false)))))))))

(fn `Ref_Actor`
  (params (Ref :type "/Game/Blueprints/PNJ/BP_Master_PNJ Object Reference"))
  (set `self.Ref_Actor_Interaction` Ref))

(fn `UserConstructionScript`)